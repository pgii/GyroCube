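; Serial port controller that streams gyro sensor readings from a COM port into the SensorController.
; It opens a fixed COM port on BeginPlay, flushes it, and closes it on EndPlay.
; Each tick it reads a pipe-delimited line and, for "gyro" messages, maps the sensor name to a bone enum and forwards the parsed quaternion to SensorController, printing a warning for unknown sensors.
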(event `self.ReceiveBeginPlay`
  (bind (_bopened _returnvalue) (`Serial.OpenComPort` 6 115200))
  (if _bopened
    (bind _output_get (set `self.SerialPort` _returnvalue))
    (`Serial.Flush` _output_get)
    (else
      (`KismetSystemLibrary.PrintString` "Port no open"))))

(event `self.ReceiveEndPlay`
  (params (EndPlayReason :type "EEndPlayReason Enum" :default "Destroyed"))
  (bind _serialport (`self.SerialPort`))
  (`/Engine/EditorBlueprintResources/StandardMacros.IsValid` _serialport
    (:`Is Valid`
      (`Serial.Close` _serialport))))

(event `self.ReceiveTick`
  (params (DeltaSeconds :type "Float (single-precision)"))
  (bind (_bsuccess _returnvalue) (`Serial.ReadString` (`self.SerialPort`)))
  (if _bsuccess
    (bind _returnvalue_2 (`KismetStringLibrary.ParseIntoArray` _returnvalue "|"))
    (if (> (`KismetArrayLibrary.Array_Length` _returnvalue_2) 0)
      (if (`KismetStringLibrary.EqualEqual_StrStr` (`|GetArrayItem` _returnvalue_2) "gyro")
        (bind _gyrosensor (`/Game/Blueprints/SensorController.GetSensorBoneEnumFromString` (`self.SensorController`) (`|GetArrayItem` _returnvalue_2 1)))
        (if (`|EnumEquality` _gyrosensor "NewEnumerator0")
          (`KismetSystemLibrary.PrintString` "Sensor not found")
          (else
            (`/Game/Blueprints/SensorController.GyroDataReceive` (`self.SensorController`) _gyrosensor (`KismetMathLibrary.MakeQuat` (`KismetStringLibrary.Conv_StringToDouble` (`|GetArrayItem` _returnvalue_2 2)) (`KismetStringLibrary.Conv_StringToDouble` (`|GetArrayItem` _returnvalue_2 3)) (`KismetStringLibrary.Conv_StringToDouble` (`|GetArrayItem` _returnvalue_2 4)) (`KismetStringLibrary.Conv_StringToDouble` (`|GetArrayItem` _returnvalue_2 5))))))))))

(fn `UserConstructionScript`)