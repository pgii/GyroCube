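; Gyro sensor motion-capture controller that turns incoming sensor quaternions into rotations for a debug cube and a T-pose mannequin.
; GyroDataReceive flips the quaternion's X and Z, then either accumulates calibration samples per sensor or applies the rotation.
; Calibration averages rotator components into a per-sensor offset, which is subtracted via DeltaRotator.
; The result drives the anim instance's single BoneRotator, with debug axes drawn for sensor, bone and offset.
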(event `GyroDataReceive`
  (params (GyroSensor :type "/Game/Blueprints/GyroSensorEnum Enum" :default "NewEnumerator0") (GyroQuaternion :type "Quat Structure"))
  (bind (_x _y _z _w) (`KismetMathLibrary.BreakQuat` GyroQuaternion))
  (bind _rotator (`self.ConvertRotator360` (`KismetMathLibrary.Quat_Rotator` (`KismetMathLibrary.MakeQuat` (* _x -1.0) (* _y 1.0) (* _z -1.0) (* _w 1.0)))))
  (if (`self.isCalibration`)
    (`self.AddCalibration` GyroSensor _rotator)
    (else
      (`self.GyroRotation` _rotator GyroSensor))))

(event `GyroRotation`
  (params (CurrentRotator :type "Rotator Structure") (GyroSensor :type "/Game/Blueprints/GyroSensorEnum Enum" :default "NewEnumerator0"))
  (bind _mesh (`Character.Mesh` (`self.TPoseCharacter`)))
  (bind _returnvalue (`SceneComponent.K2_GetComponentLocation` (`StaticMeshActor.StaticMeshComponent` (`self.CubeMesh`))))
  (bind _returnvalue_2 (`SceneComponent.K2_GetComponentLocation` (`StaticMeshActor.StaticMeshComponent` (`self.CubeMesh`))))
  (bind _returnvalue_3 (`SceneComponent.K2_GetComponentLocation` (`StaticMeshActor.StaticMeshComponent` (`self.CubeMesh`))))
  (bind _returnvalue_4 (`SceneComponent.K2_GetComponentLocation` (`StaticMeshActor.StaticMeshComponent` (`self.CubeMesh`))))
  (bind _returnvalue_5 (`SceneComponent.K2_GetComponentLocation` (`StaticMeshActor.StaticMeshComponent` (`self.CubeMesh`))))
  (bind _returnvalue_6 (`SceneComponent.K2_GetComponentLocation` (`StaticMeshActor.StaticMeshComponent` (`self.CubeMesh`))))
  ;[1 1 1] Quat axis
  (`KismetSystemLibrary.DrawDebugLine` _returnvalue (+ _returnvalue (* (`KismetMathLibrary.GetForwardVector` CurrentRotator) 250.0)) (struct :`R` 1.0 :`A` 1.0) 0.0 5.0)
  (`KismetSystemLibrary.DrawDebugLine` _returnvalue_2 (+ _returnvalue_2 (* (`KismetMathLibrary.GetUpVector` CurrentRotator) 250.0)) (struct :`B` 0.996 :`A` 1.0) 0.0 5.0)
  (`KismetSystemLibrary.DrawDebugLine` _returnvalue_3 (+ _returnvalue_3 (* (`KismetMathLibrary.GetRightVector` CurrentRotator) 250.0)) (struct :`G` 1.0 :`A` 1.0) 0.0 5.0)
  ;[1 1 1] Bone axis
  (bind _skeletonbonestruct (`self.GetSkeletonBoneStructFromSensorBone` GyroSensor))
  (bind _returnvalue_7 (`KismetStringLibrary.Conv_StringToName` (`|GetEnumeratorNameAsString` (`.SkeletonBoneEnum_2_54A5B8164DFB206B5604C6B15E9AB511` (break `/Game/Blueprints/SkeletonBoneStruct` _skeletonbonestruct)))))
  (bind _returnvalue_8 (`SceneComponent.GetSocketLocation` _mesh _returnvalue_7))
  (bind _returnvalue_9 (`SceneComponent.GetSocketRotation` _mesh _returnvalue_7))
  (`KismetSystemLibrary.DrawDebugLine` _returnvalue_8 (+ _returnvalue_8 (* (`KismetMathLibrary.GetForwardVector` _returnvalue_9) 1000.0)) (struct :`R` 1.0 :`A` 1.0) 0.0 5.0)
  (bind _returnvalue_10 (`SceneComponent.GetSocketLocation` _mesh _returnvalue_7))
  (`KismetSystemLibrary.DrawDebugLine` _returnvalue_10 (+ _returnvalue_10 (* (`KismetMathLibrary.GetUpVector` _returnvalue_9) 1000.0)) (struct :`B` 1.0 :`A` 1.0) 0.0 5.0)
  (bind _returnvalue_11 (`SceneComponent.GetSocketLocation` _mesh _returnvalue_7))
  (`KismetSystemLibrary.DrawDebugLine` _returnvalue_11 (+ _returnvalue_11 (* (`KismetMathLibrary.GetRightVector` _returnvalue_9) 1000.0)) (struct :`G` 1.0 :`A` 1.0) 0.0 5.0)
  ;[1 1 1] Offset axis
  (bind _sensoroffsetrotator (`self.GetSensorOffset` GyroSensor))
  (`KismetSystemLibrary.DrawDebugLine` _returnvalue_4 (+ _returnvalue_4 (* (`KismetMathLibrary.GetForwardVector` _sensoroffsetrotator) 250.0)) (struct :`R` 1.0 :`A` 1.0) 0.0 5.0)
  (`KismetSystemLibrary.DrawDebugLine` _returnvalue_5 (+ _returnvalue_5 (* (`KismetMathLibrary.GetUpVector` _sensoroffsetrotator) 250.0)) (struct :`B` 0.996 :`A` 1.0) 0.0 5.0)
  (`KismetSystemLibrary.DrawDebugLine` _returnvalue_6 (+ _returnvalue_6 (* (`KismetMathLibrary.GetRightVector` _sensoroffsetrotator) 250.0)) (struct :`G` 1.0 :`A` 1.0) 0.0 5.0)
  ;[1 1 1] Rotate
  (bind _rotate (`self.GetRotateOffset` GyroSensor CurrentRotator))
  (`self.K2_SetActorRotation` (`self.CubeMesh`) _rotate false)
  (`self.SetBoneRotationAnimClass` GyroSensor _rotate)
  (`KismetSystemLibrary.PrintString` (`KismetStringLibrary.Conv_RotatorToString` _rotate) true true (struct :`G` 1.0 :`A` 1.0))
  (`KismetSystemLibrary.PrintString` (`KismetStringLibrary.Conv_RotatorToString` CurrentRotator) true true (struct :`R` 1.0 :`A` 1.0)))

(fn `AddCalibration`
  (params (GyroSensor :type "/Game/Blueprints/GyroSensorEnum Enum" :default "NewEnumerator0") (Rotator :type "Rotator Structure"))
  (bind _calibrationcount (`self.GetSensorCalibrationCount` GyroSensor))
  (if (< _calibrationcount (`self.CalibrationCount`))
    (`self.AddSensorCalibrationCount` GyroSensor)
    (`self.AddSensorOffset` GyroSensor Rotator)
    (else
      (set `self.isCalibration` false)
      (bind _sensoroffsetrotator (`self.GetSensorOffset` GyroSensor))
      (`self.SetSensorOffset` GyroSensor (`KismetMathLibrary.MakeRotator` (/ (.roll _sensoroffsetrotator) (`KismetMathLibrary.Conv_IntToDouble` (`self.CalibrationCount`))) (/ (.pitch _sensoroffsetrotator) (`KismetMathLibrary.Conv_IntToDouble` (`self.CalibrationCount`))) (/ (.yaw _sensoroffsetrotator) (`KismetMathLibrary.Conv_IntToDouble` (`self.CalibrationCount`))))))))

(fn `AddSensorCalibrationCount`
  (params (GyroSensor :type "/Game/Blueprints/GyroSensorEnum Enum" :default "NewEnumerator0"))
  (returns (CalibrationCount :type Integer))
  (bind _calibrationcount (`self.GetSensorCalibrationCount` GyroSensor))
  (bind _returnvalue (+ _calibrationcount 1))
  (`BlueprintMapLibrary.Map_Add` (`self.SensorCalibrationCountMap`) GyroSensor _returnvalue)
  (return _returnvalue))

(fn `AddSensorOffset`
  (params (GyroSensor :type "/Game/Blueprints/GyroSensorEnum Enum" :default "NewEnumerator0") (AddRotator :type "Rotator Structure"))
  (returns (Rotator :type "Rotator Structure"))
  (bind _sensoroffsetrotator (`self.GetSensorOffset` GyroSensor))
  (bind _rotator (`self.SetSensorOffset` GyroSensor (`KismetMathLibrary.MakeRotator` (+ (.roll _sensoroffsetrotator) (.roll AddRotator)) (+ (.pitch _sensoroffsetrotator) (.pitch AddRotator)) (+ (.yaw _sensoroffsetrotator) (.yaw AddRotator)))))
  (return _rotator))

(fn `ConvertRotator360`
  (params (Rotation :type "Rotator Structure") (Roll :type Boolean :default true) (Pitch :type Boolean :default true) (Yaw :type Boolean :default true))
  (returns (Rotator :type "Rotator Structure"))
  (locals (localRoll :type "Float (double-precision)") (localPitch :type "Float (double-precision)") (localYaw :type "Float (double-precision)"))
  (bind _roll (.roll Rotation))
  (bind _pitch (.pitch Rotation))
  (bind _yaw (.yaw Rotation))
  (return (`KismetMathLibrary.MakeRotator` (`KismetMathLibrary.SelectFloat` (mod (+ _roll 180.0) 360.0) _roll Roll) (`KismetMathLibrary.SelectFloat` (mod (+ _pitch 180.0) 360.0) _pitch Pitch) (`KismetMathLibrary.SelectFloat` (mod (+ _yaw 180.0) 360.0) _yaw Yaw))))

(fn `GetRotateOffset`
  (params (GyroSensor :type "/Game/Blueprints/GyroSensorEnum Enum" :default "NewEnumerator0") (Rotator :type "Rotator Structure"))
  (returns (Rotate :type "Rotator Structure"))
  (`self.GetSkeletonBoneStructFromSensorBone` GyroSensor)
  (bind _sensoroffsetrotator (`self.GetSensorOffset` GyroSensor))
  (return (`KismetMathLibrary.NormalizedDeltaRotator` Rotator _sensoroffsetrotator)))

(fn `GetSensorBoneEnumFromString`
  (params (GyroSensorString :type String))
  (returns (GyroSensor :type "/Game/Blueprints/GyroSensorEnum Enum"))
  (bind _enumvalue (foreach `/Game/Blueprints/GyroSensorEnum` false)
    (:`LoopBody`
      (if (`KismetStringLibrary.EqualEqual_StrStr` (`|GetEnumeratorNameAsString` _enumvalue) GyroSensorString)
        (return _enumvalue)))
    (:`then`
      (return "NewEnumerator0"))))

(fn `GetSensorCalibrationCount`
  (params (GyroSensor :type "/Game/Blueprints/GyroSensorEnum Enum" :default "NewEnumerator0"))
  (returns (CalibrationCount :type Integer))
  (bind _sensorcalibrationcountmap (`self.SensorCalibrationCountMap`))
  (bind (_value _returnvalue) (`BlueprintMapLibrary.Map_Find` _sensorcalibrationcountmap GyroSensor))
  (if _returnvalue
    (return _value)
    (else
      (`BlueprintMapLibrary.Map_Add` _sensorcalibrationcountmap GyroSensor)
      (return 0))))

(fn `GetSensorOffset`
  (params (GyroSensor :type "/Game/Blueprints/GyroSensorEnum Enum" :default "NewEnumerator0"))
  (returns (SensorOffsetRotator :type "Rotator Structure"))
  (bind _sensoroffsetmap (`self.SensorOffsetMap`))
  (bind (_value _returnvalue) (`BlueprintMapLibrary.Map_Find` _sensoroffsetmap GyroSensor))
  (if _returnvalue
    (return _value)
    (else
      (`BlueprintMapLibrary.Map_Add` _sensoroffsetmap GyroSensor)
      (return))))

(fn `GetSkeletonBoneStructFromSensorBone`
  (params (GyroSensor :type "/Game/Blueprints/GyroSensorEnum Enum" :default "NewEnumerator0"))
  (returns (SkeletonBoneStruct :type "/Game/Blueprints/SkeletonBoneStruct Structure"))
  (bind (_value _returnvalue) (`BlueprintMapLibrary.Map_Find` (`self.SensorSkeletonBoneMapStruct`) GyroSensor))
  (if _returnvalue
    (return _value)
    (else
      (return (make `/Game/Blueprints/SkeletonBoneStruct` "NewEnumerator0")))))

(fn `ResetAllSensorCalibrationCount`
  (bind _enumvalue (foreach `/Game/Blueprints/GyroSensorEnum` false)
    (:`LoopBody`
      (`BlueprintMapLibrary.Map_Add` (`self.SensorCalibrationCountMap`) _enumvalue))
    (:`then`
      (return))))

(fn `ResetAllSensorOffset`
  (bind _enumvalue (foreach `/Game/Blueprints/GyroSensorEnum` false)
    (:`LoopBody`
      (`BlueprintMapLibrary.Map_Add` (`self.SensorOffsetMap`) _enumvalue))
    (:`then`
      (return))))

(fn `SetBoneRotationAnimClass`
  (params (GyroSensor :type "/Game/Blueprints/GyroSensorEnum Enum" :default "NewEnumerator0") (Rotator :type "Rotator Structure"))
  (returns (BoneName :type Name) (Rotate :type "Rotator Structure"))
  (bind _skeletonbonestruct (`self.GetSkeletonBoneStructFromSensorBone` GyroSensor))
  (`self.GetSensorOffset` GyroSensor)
  (bind _assk_mannequin_mocap_anim_bp (cast `/Game/Character/SK_MannequinMocapAnim_BP` (`SkeletalMeshComponent.GetAnimInstance` (`Character.Mesh` (`self.TPoseCharacter`)))))
  (set `/Game/Character/SK_MannequinMocapAnim_BP.BoneRotator` Rotator _assk_mannequin_mocap_anim_bp)
  (return (`KismetStringLibrary.Conv_StringToName` (`|GetEnumeratorNameAsString` (`.SkeletonBoneEnum_2_54A5B8164DFB206B5604C6B15E9AB511` (break `/Game/Blueprints/SkeletonBoneStruct` _skeletonbonestruct)))) Rotator))

(fn `SetSensorOffset`
  (params (GyroSensor :type "/Game/Blueprints/GyroSensorEnum Enum" :default "NewEnumerator0") (AddRotator :type "Rotator Structure"))
  (returns (Rotator :type "Rotator Structure"))
  (`BlueprintMapLibrary.Map_Add` (`self.SensorOffsetMap`) GyroSensor AddRotator)
  (return AddRotator))

(fn `UserConstructionScript`)